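; BP_carSpawner periodically spawns traffic vehicles at its own transform.
; On BeginPlay it starts a looping timer with a random interval, rolled once per spawner.
; Nested FlipFlops make every other spawn a van, with the spawns between alternating between two car models.
; Each vehicle receives random picks from the StartPoints and EndPoints arrays as its route endpoints.
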(event `self.ReceiveBeginPlay`
  (`KismetSystemLibrary.K2_SetTimerDelegate` (delegate `Spawn`) (`KismetMathLibrary.RandomFloatInRange` 1.0 5.0) true))

(event `Spawn`
  (`/Engine/EditorBlueprintResources/StandardMacros.FlipFlop`
    (:`A`
      (`/Engine/EditorBlueprintResources/StandardMacros.FlipFlop`
        (:`A`
          (`|SpawnActorFromClass` "/Game/Fab/Assets/Cartoon_City_Free/Actors/SM_Car_19.SM_Car_19_C" (`self.GetTransform`) "Undefined" "MultiplyWithRoot" null (`KismetArrayLibrary.Array_Random` (`self.StartPoints`)) (`KismetArrayLibrary.Array_Random` (`self.EndPoints`)) null))
        (:`B`
          (`|SpawnActorFromClass` "/Game/Fab/Assets/Cartoon_City_Free/Actors/SM_Car_06.SM_Car_06_C" (`self.GetTransform`) "Undefined" "MultiplyWithRoot" null (`KismetArrayLibrary.Array_Random` (`self.StartPoints`)) (`KismetArrayLibrary.Array_Random` (`self.EndPoints`)) null))))
    (:`B`
      (`|SpawnActorFromClass` "/Game/Fab/Assets/Cartoon_City_Free/Actors/SM_Van.SM_Van_C" (`self.GetTransform`) "Undefined" "MultiplyWithRoot" null (`KismetArrayLibrary.Array_Random` (`self.StartPoints`)) (`KismetArrayLibrary.Array_Random` (`self.EndPoints`)) null))))

(fn `UserConstructionScript`)