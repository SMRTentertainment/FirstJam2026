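; Base NPC character that travels in a straight line toward an End actor until something overlaps it and knocks it into a ragdoll.
; Tick moves it by setting the actor location at a constant Speed without sweeping, rather than through CharacterMovement.
; The first capsule overlap, from any source, disables movement, enables mesh physics and launches it in a random direction, then destroys the actor after a short delay.
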(event `self.ReceiveBeginPlay`
  (`self.K2_SetActorLocation` (`self.K2_GetActorLocation`)))

(event `self.ReceiveTick`
  (params (DeltaSeconds :type "Float (single-precision)"))
  (if (not (`self.IsRagdoll`))
    (`self.K2_SetActorLocation` (+ (`self.K2_GetActorLocation`) (* (* (`KismetMathLibrary.Normal` (- (`self.K2_GetActorLocation` (`self.End`)) (`self.K2_GetActorLocation`))) (`self.Speed`)) DeltaSeconds)))))

(event `self.CapsuleComponent.OnComponentBeginOverlap`
  (params (OverlappedComponent :type "PrimitiveComponent Object Reference") (OtherActor :type "Actor Object Reference") (OtherComp :type "PrimitiveComponent Object Reference") (OtherBodyIndex :type Integer) (bFromSweep :type Boolean) (SweepResult :type "HitResult Structure (by ref)"))
  (bind _mesh (`self.Mesh`))
  (if (not (`self.IsRagdoll`))
    (set `self.IsRagdoll` true)
    (`CharacterMovementComponent.DisableMovement` (`self.CharacterMovement`))
    (`PrimitiveComponent.SetSimulatePhysics` _mesh true)
    (`PrimitiveComponent.SetCollisionProfileName` _mesh "Ragdoll" true)
    (`PrimitiveComponent.AddImpulse` (`self.Mesh`) (* (`KismetMathLibrary.RandomUnitVector`) 1250.0) "None" true)
    (`KismetSystemLibrary.Delay` 4.0)
    (`self.K2_DestroyActor`)))

(fn `UserConstructionScript`)